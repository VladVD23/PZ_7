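; AI spawner actor that spawns a ThirdPersonCharacter at its own location with zero rotation.
; BeginPlay calls SpawnAI once, which spawns only with authority and when time since creation exceeds the last spawn time plus a cooldown.
; A valid spawn records the time.
; SpawnAI returns true after any spawn attempt, even a failed one, and false on remotes or during cooldown.
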(event EventBeginPlay
  (CallFunction|SpawnAI))

(fn ConstructionScript)

(fn SpawnAI
  (Networking|SwitchHasAuthority
    (:Authority
      (if (> (Actor|GetGameTimeSinceCreation) (+ (Variables|Default|GetLastTimeSpawned) (Variables|Default|GetSpawnCooldown)))
        (bind _returnvalue (Game|SpawnActorfromClass "/Game/ThirdPersonBP/Blueprints/ThirdPersonCharacter.ThirdPersonCharacter_C" (Math|Transform|MakeTransform (Transformation|GetActorLocation)) "Undefined" 0 0))
        (Utilities|IsValid _returnvalue
          (:Is%20Valid
            (Variables|Default|SetLastTimeSpawned (Actor|GetGameTimeSinceCreation))
            (return true))
          (:Is%20Not%20Valid
            (return true)))
        (else
          (return false))))
    (:Remote
      (return false))))