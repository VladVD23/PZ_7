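; BP_MyGameMode is a game mode that spawns AI through the level's BP_AISpawner actors.
; SpawnAI shuffles the spawner list and tries each until one reports success, giving a random spawn location.
; LazyGetAISpawners is meant to cache that list, but as wired it queries the world only when SpawnersFound is already true.
; BeginPlay and Tick are unused, and nothing in this Blueprint calls SpawnAI.
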(event EventBeginPlay)

(event EventTick
  (params (DeltaSeconds :type Float%20%28single-precision%29)))

(fn ConstructionScript)

(fn LazyGetAISpawners
  (Utilities|FlowControl|Sequence
    (:then_0
      (if (Variables|Default|GetSpawnersFound)
        (bind _outactors (Actor|GetAllActorsOfClass "/Game/BP_AISpawner.BP_AISpawner_C"))
        (Variables|Default|SetOutActors _outactors)
        (Variables|Default|SetSpawnersFound true)))
    (:then_1
      (return (Variables|Default|GetOutActors)))))

(fn SpawnAI
  (bind _outactors (CallFunction|LazyGetAISpawners))
  (bind _output_get (LocalVariables|SetL_Spawners _outactors))
  (Utilities|Array|Shuffle _output_get)
  (bind _array_element (Utilities|Array|ForEachLoopwithBreak _output_get :!label _label)
    (:LoopBody
      (bind _result (Default|SpawnAI _array_element))
      (if _result
        (goto _label Break)))
    (:Completed
      (return))))